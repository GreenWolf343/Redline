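; Race tracker that manages a level's checkpoint sequence, laps and race completion through Redline_PlayerController.
; On BeginPlay it passes map, lap, save and medal-time settings to the controller, then numbers the Checkpoints array, activates the first and starts music.
; Each cleared-checkpoint callback plays a sound, activates the next checkpoint and moves the respawn point.
; The last checkpoint updates the lap, wrapping to the first until MaxLaps is reached, when the controller's Restart is called.
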(event `self.ReceiveBeginPlay`
  ;[1 0.7886 0.04201] Begin Play
  (bind _asredline_player_controller (cast `/Game/Redline_Project/Blueprints/Redline_PlayerController` (`GameplayStatics.GetPlayerController` 0)))
  (set `self.ControllerRef` _asredline_player_controller)
  (`self.ApplySettings`)
  (`self.StartSequence`))

(event `ApplySettings`
  (bind _controllerref (`self.ControllerRef`))
  ;[1 0.7886 0.04201] Apply User Settings
  (set `/Game/Redline_Project/Blueprints/Redline_PlayerController.MaxLaps` (`self.MaxLaps`) _controllerref)
  (set `/Game/Redline_Project/Blueprints/Redline_PlayerController.SaveSlot` (`self.SaveGameName`) _controllerref)
  (set `/Game/Redline_Project/Blueprints/Redline_PlayerController.NameOfMapText` (`self.NameMap`) _controllerref)
  (`self.UpdateTimers`)
  (`/Game/Redline_Project/Blueprints/Redline_PlayerController.StartGameSetup` _controllerref))

(event `StartSequence`
  (bind _checkpoints (`self.Checkpoints`))
  ;[1 0.7886 0.04201] Start Sequence
  (for (_array_element _array_index) (`self.Checkpoints`)
    (set `/Game/Redline_Project/Blueprints/Checkpoint_BP.CheckpointNumber` (+ _array_index 1) _array_element)
    (set `self.TotalCheckpoints` (`KismetArrayLibrary.Array_Length` _checkpoints))
    (`self.ActivateCheckpoint` (`|GetArrayItem` _checkpoints))
    (for _array_element_2 (`self.Checkpoints`)
      (add `/Game/Redline_Project/Blueprints/Checkpoint_BP.CheckpointCleared` _array_element_2 (delegate `Checkpoint Cleared`))
      (`AudioComponent.Play` (`AmbientSound.AudioComponent` (`self.Level Music`)) 0.0))))

(event `Checkpoint Cleared`
  (params (NextCheckpoint :type Integer))
  (bind _controllerref (`self.ControllerRef`))
  ;[1 0.7886 0.04201] Clear Checkpoints
  (`self.LapCheck` NextCheckpoint)
  (`AudioComponent.Play` (`AmbientSound.AudioComponent` (`self.Checkpoint Sound`)) 0.0)
  (if (`/Game/Redline_Project/Blueprints/Redline_PlayerController.RaceComplete?` _controllerref)
    (`/Game/Redline_Project/Blueprints/Redline_PlayerController.Restart` _controllerref)))

(fn `ActivateCheckpoint`
  (params (NextCheckpoint :type "/Game/Redline_Project/Blueprints/Checkpoint_BP Object Reference"))
  (bind _checkpointtrigger (`/Game/Redline_Project/Blueprints/Checkpoint_BP.CheckpointTrigger` NextCheckpoint))
  ;[1 1 1] Activates the next Checkpoint
  (`SceneComponent.SetHiddenInGame` _checkpointtrigger false false)
  (`SceneComponent.SetHiddenInGame` (`/Game/Redline_Project/Blueprints/Checkpoint_BP.ParticleSystem` NextCheckpoint) false false)
  (set `PrimitiveComponent.bGenerateOverlapEvents` true _checkpointtrigger))

(fn `LapCheck`
  (params (Checkpoint :type Integer))
  (locals (LocalCheckpoint :type Integer))
  ;[1 1 1] Comment
  (bind _output_get (set `local.LocalCheckpoint` Checkpoint))
  (if (== _output_get (`self.TotalCheckpoints`))
    (bind _isracecomplete_ (`self.RaceCompleteCheck`))
    (if (not _isracecomplete_)
      (`self.ActivateCheckpoint` (`|GetArrayItem` (`self.Checkpoints`))))
    (`/Game/Redline_Project/Blueprints/Redline_PlayerController.UpdateLap` (`self.ControllerRef`))
    (else
      (`self.ActivateCheckpoint` (`|GetArrayItem` (`self.Checkpoints`) (`local.LocalCheckpoint`)))))
  (set `/Game/Redline_Project/Blueprints/Redline_PlayerController.RespawnLocation` (`self.GetTransform` (`|GetArrayItem` (`self.Checkpoints`) (- (`local.LocalCheckpoint`) 1))) (`self.ControllerRef`)))

(fn `RaceCompleteCheck`
  (returns (`IsRaceComplete?` :type Boolean))
  (locals (LocalComplete :type Boolean))
  (bind _controllerref (`self.ControllerRef`))
  (bind _controllerref_2 (`self.ControllerRef`))
  ;[1 1 1] Race Complete Checks
  (if (>= (`/Game/Redline_Project/Blueprints/Redline_PlayerController.ActualLap` _controllerref_2) (`/Game/Redline_Project/Blueprints/Redline_PlayerController.MaxLaps` _controllerref_2))
    (bind _output_get (set `/Game/Redline_Project/Blueprints/Redline_PlayerController.RaceComplete?` true _controllerref))
    (set `local.LocalComplete` _output_get)
    (else
      (bind _output_get_2 (set `/Game/Redline_Project/Blueprints/Redline_PlayerController.RaceComplete?` false _controllerref))
      (set `local.LocalComplete` _output_get_2)))
  (return (`local.LocalComplete`)))

(fn `UpdateTimers`
  (bind _controllerref (`self.ControllerRef`))
  ;[1 1 1] Pass User Times To Redline Controller Times
  (set `/Game/Redline_Project/Blueprints/Redline_PlayerController.GoldTime` (`self.GoldTime`) _controllerref)
  (set `/Game/Redline_Project/Blueprints/Redline_PlayerController.SilverTime` (`self.SilverTime`) _controllerref)
  (set `/Game/Redline_Project/Blueprints/Redline_PlayerController.BronzeTime` (`self.BronzeTime`) _controllerref)
  (set `/Game/Redline_Project/Blueprints/Redline_PlayerController.DefaultBestLapTime` (`self.DefaultBestLap`) _controllerref)
  (set `/Game/Redline_Project/Blueprints/Redline_PlayerController.DefaultBestRaceTime` (`self.DefaultBestTime`) _controllerref))

(fn `UserConstructionScript`)