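; Player controller for the Redline racing game that creates the HUD, caches the player's vehicle and tracks laps.
; RespawnVehicle spawns a new vehicle at the stored respawn transform and possesses it.
; UpdateLap increments and prints the lap count until the race completes, then calls the lap time check.
; Timers, restart, save/load, goal updates and time checks are empty stubs.
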(event `self.ReceiveBeginPlay`
  ;[1 0.7785 0] Event Begin Play / Get Ref
  (bind _returnvalue (`|CreateWidget` "/Game/Redline_Project/Blueprints/UI/Redline_HUD.Redline_HUD_C"))
  (bind _output_get (set `self.HUDRef` _returnvalue))
  (`UserWidget.AddToViewport` _output_get 0)
  (bind _asvehicle_blueprint (cast `/Game/Redline_Project/Blueprints/Car/VehicleBlueprint` (`GameplayStatics.GetPlayerPawn` 0)))
  (set `self.VehicleRef` _asvehicle_blueprint))

(event `StartGameSetup`)

(event `StartRaceTime`)

(event `StopRaceTime`)

(event `Restart`)

(event `StartLapTime`)

(event `StopLapTime`)

(event `RespawnVehicle`
  ;[1 1 1] Respawn Vehicle
  (bind _returnvalue (`|SpawnActorFromClass` "/Game/Redline_Project/Blueprints/Car/VehicleBlueprint.VehicleBlueprint_C" (`self.RespawnLocation`) "Undefined" "OverrideRootScale" null null))
  (`self.Possess` _returnvalue))

(event `UpdateLap`
  ;[1 1 1] Update Lap - Checks New Lap Record
  (if (not (`self.RaceComplete?`))
    (bind _output_get (set `self.ActualLap` (+ (`self.ActualLap`) 1)))
    (bind _output_get_2 (set `self.CurrentLapText` (`KismetTextLibrary.Conv_IntToText` _output_get))))
  (`self.LapTimeCheck`)
  (`KismetSystemLibrary.PrintText` _output_get_2))

(fn `InitText`)

(fn `LapTimeCheck`)

(fn `LoadTheGame`)

(fn `RaceTimeCheck`)

(fn `SaveGameCheck`)

(fn `SaveTheGame`)

(fn `UpdateGoals`)

(fn `UserConstructionScript`)